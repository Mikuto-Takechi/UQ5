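; GA_ThrowBomb is a gameplay ability that plays the throw montage and can hold it mid-animation.
; While a gate is open, a montage notify pauses the montage.
; An Ability.State.End gameplay event resumes the montage, closes the gate and ends the ability.
; The ability also ends when the montage completes, blends out or is interrupted; the graph itself spawns no bomb.
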(event `self.K2_ActivateAbility`
  (bind _returnvalue (`self.GetOwningComponentFromActorInfo`))
  (bind _returnvalue_2 (`SkeletalMeshComponent.GetAnimInstance` _returnvalue))
  (`AbilityTask_WaitGameplayEvent.WaitGameplayEvent` (struct :`TagName` "Ability.State.End") null true
    (:`then`
      (bind _notifyname (`|PlayMontage` _returnvalue "/Game/UnrealQuest5/Characters/Mannequins/Animations/UQ5/AM_Throw.AM_Throw")
        (:`then`
          (goto _label_2 :!via `Open`))
        (:`OnCompleted`
          (`self.K2_EndAbility` :!label _label))
        (:`OnBlendOut`
          (goto _label))
        (:`OnInterrupted`
          (goto _label))
        (:`OnNotifyBegin`
          (switch `name` _notifyname
            (:`Pause`
              (`/Engine/EditorBlueprintResources/StandardMacros.Gate` true :!label _label_2
                (:`Exit`
                  (`AnimInstance.Montage_Pause` _returnvalue_2 "/Game/UnrealQuest5/Characters/Mannequins/Animations/UQ5/AM_Throw.AM_Throw"))))))))
    (:`EventReceived`
      (`AnimInstance.Montage_Resume` _returnvalue_2 "/Game/UnrealQuest5/Characters/Mannequins/Animations/UQ5/AM_Throw.AM_Throw")
      (`|ExecutionSequence`
        (:`then_0`
          (goto _label_2 :!via `Close`))
        (:`then_1`
          (`self.K2_EndAbility`))))))