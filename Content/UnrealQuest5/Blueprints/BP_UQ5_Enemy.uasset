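; BP_UQ5_Enemy is a sword-wielding enemy that attacks the player, can be parried and takes hits.
; Attack montage notifies trigger damage to players overlapping AttackArea and toggle the CanParry window; GotParried closes it and plays a reaction.
; OnHit layers a damage montage, decrements HitPoint and is meant to pause and later resume an interrupted attack.
; At zero HitPoint it ragdolls, drops its blade and is destroyed after a timer.
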(event `GotParried`
  (`GameplayStatics.PlaySoundAtLocation` "/Game/UnrealQuest5/Sound/剣で打ち合う2.剣で打ち合う2" (`self.K2_GetActorLocation`) (struct) 1.0 1.0 0.0 null null null null)
  (set `self.CanParry` false)
  (`KismetSystemLibrary.PrintString` "Got Parried")
  (`|PlayMontage` (`self.Mesh`) "/Game/UnrealQuest5/Characters/Mannequins/Animations/UQ5/AM_GotParried.AM_GotParried"))

(event `Attack`
  ;[1 0 0 0.5] 攻撃
  (bind _notifyname (`|PlayMontage` (`self.Mesh`) "/Game/UnrealQuest5/Characters/Mannequins/Animations/UQ5/AM_Enemy_Attack01.AM_Enemy_Attack01")
    (:`OnNotifyBegin`
      (`self.EnemyAttack` _notifyname))
    (:`OnNotifyEnd`
      _))
  (`self.Parry` _notifyname))

(event `Ragdoll`
  (bind _mesh (`self.Mesh`))
  (bind _blademesh (`self.BladeMesh`))
  (`PrimitiveComponent.SetSimulatePhysics` _mesh true)
  (`PrimitiveComponent.SetCollisionEnabled` _mesh "PhysicsOnly")
  (`PrimitiveComponent.SetCollisionEnabled` (`self.CapsuleComponent`) "NoCollision")
  (`CharacterMovementComponent.DisableMovement` (`self.CharacterMovement`))
  (`SceneComponent.K2_DetachFromComponent` _blademesh "KeepWorld" "KeepWorld" "KeepWorld" true)
  (`PrimitiveComponent.SetSimulatePhysics` _blademesh true)
  (`PrimitiveComponent.SetCollisionEnabled` _blademesh "PhysicsOnly")
  (`KismetSystemLibrary.K2_SetTimer` null "Dispose" 3.0))

(event `OnHit`
  (bind _returnvalue (`SkeletalMeshComponent.GetAnimInstance` (`self.Mesh`)))
  (if (> (`self.HitPoint`) 0)
    (`GameplayStatics.PlaySoundAtLocation` "/Game/UnrealQuest5/Sound/剣で斬る1.剣で斬る1" (`self.K2_GetActorLocation`) (struct) 1.0 1.0 0.0 null null null null)
    (if (== _returnvalue "/Game/UnrealQuest5/Characters/Mannequins/Animations/UQ5/AM_Enemy_Attack01.AM_Enemy_Attack01")
      (`AnimInstance.Montage_Pause` _returnvalue "/Game/UnrealQuest5/Characters/Mannequins/Animations/UQ5/AM_Enemy_Attack01.AM_Enemy_Attack01")
      (set `self.ResumeAttack` true) ; 攻撃再開用のフラグをtrueにする
    )
    (bind _returnvalue_2 (`AnimInstance.Montage_Play` _returnvalue "/Game/UnrealQuest5/Characters/Mannequins/Animations/UQ5/AM_Damaged.AM_Damaged" 1.0 "MontageLength" 0.0 false)) ; PlayMontageだと前に再生されていたモンタージュがなくなってしまうのでこれを使う
    (`|ExecutionSequence`
      (:`then_0`
        ;[1 1 1] ダメージ計算＆処理
        (set `self.HitPoint` (- (`self.HitPoint`) 1))
        (if (<= (`self.HitPoint`) 0)
          (`/Engine/EditorBlueprintResources/StandardMacros.DoOnce` false
            (:`Completed`
              (`self.Ragdoll`)))))
      (:`then_1`
        ;[1 1 1] 攻撃再開処理
        (`KismetSystemLibrary.Delay` _returnvalue_2)
        (if (`self.ResumeAttack`)
          (set `self.ResumeAttack` false)
          (`AnimInstance.Montage_Resume` (`SkeletalMeshComponent.GetAnimInstance` (`self.Mesh`)) "/Game/UnrealQuest5/Characters/Mannequins/Animations/UQ5/AM_Enemy_Attack01.AM_Enemy_Attack01"))))))

(fn `Dispose`
  (`self.K2_DestroyActor`))

(fn `EnemyAttack`
  (params (`Notify Name` :type Name))
  (if (== `Notify Name` "EnemyAttack")
    (for _array_element (`PrimitiveComponent.GetOverlappingActors` (`self.AttackArea`) "/Game/UnrealQuest5/Blueprints/BP_UQ5_Player.BP_UQ5_Player_C")
      (bind _asbp_uq5_player (cast `/Game/UnrealQuest5/Blueprints/BP_UQ5_Player` _array_element))
      (`/Game/UnrealQuest5/Blueprints/BP_UQ5_Player.OnHit` _asbp_uq5_player))))

(fn `Parry`
  (params (`Notify Name` :type Name))
  (if (== `Notify Name` "CanParry")
    (if (== (`self.CanParry`) true)
      (set `self.CanParry` false)
      (else
        (set `self.CanParry` true)))))

(fn `UserConstructionScript`)